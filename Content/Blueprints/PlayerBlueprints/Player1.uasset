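; Player1 is a player-flown spaceship with six-axis flight, two switchable weapons, shields and hull.
; Input events add linear and angular velocity to the physics capsule only on authority, with gravity off and damping on.
; Lasers (once per press) and delayed gatling guns line-trace forward, damaging asteroids via multicast and other players via ApplyDamage, alongside attached particle effects.
; Damage drains shields, then hull; Tick swaps a dead ship for explosion actors.
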(event Custom|CheckIfPlayerDied
  ;[1 1 1] Server handles clients input ONLY on authority machine
  (if (not (> (Variables|Default|GetShipHullIntegrity) 0.0))
    (Game|SpawnActorfromClass "/Game/Blueprints/PartcileBluePrints/Blueprint_Effect_Explosion.Blueprint_Effect_Explosion_C" (Math|Conversions|ToTransform(Vector) (Transformation|GetActorLocation)) false 0)
    (Actor|DestroyActor)
    (Game|SpawnActorfromClass "/Game/Blueprints/PlayerBlueprints/ExplodingPlayer.ExplodingPlayer_C" (Transformation|GetActorTransform) false 0)))

(event Custom|Stop%20Player
  ;[1 1 1] Server handles clients input ONLY on authority machine
  (Variables|PhysicsValues|SetForwardSpeed 0.0))

(event Custom|Input%20Forward
  (params (Axis%20Value :type Float%20%28single-precision%29))
  ;[1 1 1] Server handles clients input ONLY on authority machine
  (Networking|SwitchHasAuthority
    (:Authority
      (Variables|PhysicsValues|SetForwardSpeed (Math|Float|Clamp(Float) (+ Axis%20Value (Variables|PhysicsValues|GetForwardSpeed)) -1e+02 1e+02))
      (Class|PrimitiveComponent|SetAllPhysicsLinearVelocity (Variables|Collision|GetCapsuleComponent) (* (Transformation|GetActorForwardVector) (Variables|PhysicsValues|GetForwardSpeed)) true))))

(event Custom|InputLateral
  (params (Axis%20Value :type Float%20%28single-precision%29))
  ;[1 1 1] Server handles clients input ONLY on authority machine
  (Networking|SwitchHasAuthority
    (:Authority
      (Class|PrimitiveComponent|SetAllPhysicsLinearVelocity (Variables|Collision|GetCapsuleComponent) (* (Transformation|GetActorRightVector) (* Axis%20Value (Variables|PhysicsValues|GetAccel))) true))))

(event Custom|Switch%20Weapon
  (params (WeaponToSwitchTo :type Integer))
  ;[1 1 1] Server handles clients input ONLY on authority machine
  (Variables|Default|SetWeaponSelection WeaponToSwitchTo))

(event Custom|PlayerMouseUpEvent
  ;[1 1 1] Server handles clients input ONLY on authority machine
  (switch int (Variables|Default|GetWeaponSelection)
    (:0
      (CallFunction|ResetShooting)
      (Utilities|FlowControl|Delay 5.0)
      (Components|DestroyComponent (stale Custom|PlayerMouseDownEvent _returnvalue))
      (Components|DestroyComponent (stale Custom|PlayerMouseDownEvent _returnvalue_2)))
    (:1
      (Components|Activation|Deactivate (Variables|Default|GetBulletParticle1))
      (Components|Activation|Deactivate (Variables|Default|GetBulletParticle2)))))

(event Custom|PlayerMouseDownEvent
  ;[1 1 1] Server handles clients input ONLY on authority machine
  (switch int (Variables|Default|GetWeaponSelection)
    (:0
      (bind _returnvalue (Effects|SpawnEmitterAttached "/Game/Particles/P_Lasers.P_Lasers" (Variables|Default|GetLaser1) "None"))
      (Effects|Components|ParticleSystem|SetColorParameter _returnvalue "ParticleColor" "(R=1.000000,G=0.000000,B=0.000000,A=1.000000)")
      (bind _returnvalue_2 (Effects|SpawnEmitterAttached "/Game/Particles/P_Lasers.P_Lasers" (Variables|Default|GetLaser2) "None"))
      (Effects|Components|ParticleSystem|SetColorParameter _returnvalue_2 "ParticleColor" "(R=1.000000,G=0.000000,B=0.000000,A=1.000000)"))
    (:1
      (Components|Activation|Activate (Variables|Default|GetBulletParticle1) false)
      (Components|Activation|Activate (Variables|Default|GetBulletParticle2) false))))

(event Custom|ShootMainWeapon
  ;[1 1 1] Server handles clients input ONLY on authority machine
  (switch int (Variables|Default|GetWeaponSelection)
    (:0
      (Utilities|FlowControl|DoOnce false
        (:Completed
          (bind _outhit (Collision|LineTraceForObjects (Transformation|GetActorLocation) (+ (* (Transformation|GetActorForwardVector) 5e+03) (Transformation|GetActorLocation)) (Utilities|Array|MakeArray "ObjectTypeQuery4" "ObjectTypeQuery6") false 0 "None"))
          (Variables|Default|SetLineTraceHitLocation (.Location (Collision|BreakHitResult _outhit)))
          (Variables|Default|SetLineTraceHitNormal (.ImpactNormal (Collision|BreakHitResult _outhit)))
          (if (== (Utilities|GetClass (.HitActor (Collision|BreakHitResult _outhit))) "/Game/Blueprints/SceneObjectBlueprints/DM_Asteroid.DM_Asteroid_C")
            (bind _asdm_asteroid (Utilities|Casting|CastToDM_Asteroid (.HitActor (Collision|BreakHitResult _outhit)))
              (:then
                (Default|MulticastDamage _asdm_asteroid (Variables|Default|GetLaserDamage) (Variables|Default|GetLineTraceHitLocation) (* (Variables|Default|GetLineTraceHitNormal) -1.0)))
              (:CastFailed
                (Development|PrintString "The cast in player1 script FAILED")))
            (elif (== (Utilities|GetClass (.HitActor (Collision|BreakHitResult _outhit))) "Player1_C")
              (Game|Damage|ApplyDamage (.HitActor (Collision|BreakHitResult _outhit)) (Variables|Default|GetLaserDamage) 0 0))))))
    (:1
      (Utilities|FlowControl|Delay 0.3)
      (bind _outhit_2 (Collision|LineTraceForObjects (Transformation|GetActorLocation) (+ (* (Transformation|GetActorForwardVector) 5e+03) (Transformation|GetActorLocation)) (Utilities|Array|MakeArray "ObjectTypeQuery4" "ObjectTypeQuery6") false 0 "None"))
      (Variables|Default|SetLineTraceHitLocation (.Location (Collision|BreakHitResult _outhit_2)))
      (Variables|Default|SetLineTraceHitNormal (.ImpactNormal (Collision|BreakHitResult _outhit_2)))
      (if (== (Utilities|GetClass (.HitActor (Collision|BreakHitResult _outhit_2))) "/Game/Blueprints/SceneObjectBlueprints/DM_Asteroid.DM_Asteroid_C")
        (bind _asdm_asteroid_2 (Utilities|Casting|CastToDM_Asteroid (.HitActor (Collision|BreakHitResult _outhit_2)))
          (:then
            (Default|MulticastDamage _asdm_asteroid_2 (Variables|Default|GetLaserDamage) (Variables|Default|GetLineTraceHitLocation) (* (Variables|Default|GetLineTraceHitNormal) -1.0)))
          (:CastFailed
            (Development|PrintString "The cast in player1 script FAILED")))
        (elif (== (Utilities|GetClass (.HitActor (Collision|BreakHitResult _outhit_2))) "Player1_C")
          (Game|Damage|ApplyDamage (.HitActor (Collision|BreakHitResult _outhit_2)) (Variables|Default|GetBulletDamage) 0 0))))))

(event Custom|ResetShooting
  ;[1 1 1] Server handles clients input ONLY on authority machine
  (Utilities|FlowControl|DoOnce false) ; enters at Reset
)

(event Custom|InputVertical
  (params (Axis%20Value :type Float%20%28single-precision%29))
  ;[1 1 1] Server handles clients input ONLY on authority machine
  (Networking|SwitchHasAuthority
    (:Authority
      (Class|PrimitiveComponent|SetAllPhysicsLinearVelocity (Variables|Collision|GetCapsuleComponent) (* (Transformation|GetActorUpVector) (* Axis%20Value (Variables|PhysicsValues|GetAccel))) true))))

(event Custom|Pitch
  (params (Pitch :type Float%20%28single-precision%29))
  ;[1 1 1] Server handles clients input ONLY on authority machine
  (Networking|SwitchHasAuthority
    (:Authority
      (Class|PrimitiveComponent|SetPhysicsAngularVelocity (Variables|Collision|GetCapsuleComponent) (* (Transformation|GetActorRightVector) (* Pitch (Variables|PhysicsValues|GetTurn%20speed) 0.3)) true "None"))))

(event Custom|Yaw
  (params (Yaw :type Float%20%28single-precision%29))
  ;[1 1 1] Server handles clients input ONLY on authority machine
  (Networking|SwitchHasAuthority
    (:Authority
      (Class|PrimitiveComponent|SetPhysicsAngularVelocity (Variables|Collision|GetCapsuleComponent) (* (Transformation|GetActorUpVector) (* Yaw (Variables|PhysicsValues|GetTurn%20speed) 0.5)) true "None"))))

(event Custom|Roll
  (params (Roll :type Float%20%28single-precision%29))
  ;[1 1 1] Server handles clients input ONLY on authority machine
  (Networking|SwitchHasAuthority
    (:Authority
      (Class|PrimitiveComponent|SetPhysicsAngularVelocity (Variables|Collision|GetCapsuleComponent) (* (Transformation|GetActorForwardVector) (* Roll (Variables|PhysicsValues|GetTurn%20speed) 3.0)) true "None"))))

(event EventAnyDamage
  (params (Damage :type Float%20%28single-precision%29) (DamageType :type Damage%20Type%20Object%20Reference) (InstigatedBy :type Controller%20Object%20Reference) (DamageCauser :type Actor%20Object%20Reference))
  ;[1 1 1] Server handles clients input ONLY on authority machine
  (if (and (!= (Variables|Default|GetShields) 0.0) (> (Variables|Default|GetShields) 0.0))
    (Variables|Default|SetShields (- (Variables|Default|GetShields) Damage))
    (else
      (Variables|Default|SetShipHullIntegrity (- (Variables|Default|GetShipHullIntegrity) Damage)))))

(event EventBeginPlay
  (Utilities|FlowControl|Sequence
    (:then_0
      ;[1 1 1] Every tick
      (bind _asmy_game_instance (Utilities|Casting|CastToMyGameInstance (Game|GetGameInstance)))
      (Variables|Default|SetGameInstance _asmy_game_instance))
    (:then_1
      (bind _returnvalue (Effects|SpawnEmitterAttached "/Game/Particles/P_Bullets.P_Bullets" (Variables|Default|GetBullet1) "None" "0, 0, 0" "0, 0, 0" "KeepRelativeOffset" false))
      (Components|Activation|Deactivate _returnvalue)
      (Variables|Default|SetBulletParticle1 _returnvalue)
      (bind _returnvalue_2 (Effects|SpawnEmitterAttached "/Game/Particles/P_Bullets.P_Bullets" (Variables|Default|GetBullet2) "None" "0, 0, 0" "0, 0, 0" "KeepRelativeOffset" false))
      (Components|Activation|Deactivate _returnvalue_2)
      (Variables|Default|SetBulletParticle2 _returnvalue_2))
    (:then_2
      (Physics|SetEnableGravity (Variables|Collision|GetCapsuleComponent) false)
      (Class|PrimitiveComponent|SetAngularDamping (Variables|Collision|GetCapsuleComponent) 3.0)
      (Class|PrimitiveComponent|SetLinearDamping (Variables|Collision|GetCapsuleComponent) 6.0))))

(event EventTick
  (params (DeltaSeconds :type Float%20%28single-precision%29))
  ;[1 1 1] Every tick
  (Networking|SwitchHasAuthority
    (:Authority
      _)
    (:Remote
      _))
  (CallFunction|CheckifPlayerDied))

(event Input|ActionEvents|InputActionSwitchWeapon1
  ;[1 1 1] Client Inputs Values
  (:Pressed
    (CallFunction|SwitchWeapon)
    (Development|PrintString "Switched To lasors" true true "(R=1.000000,G=0.000000,B=0.040099,A=1.000000)")))

(event Input|ActionEvents|InputActionSwitchWeapon2
  ;[1 1 1] Client Inputs Values
  (:Pressed
    (CallFunction|SwitchWeapon 1)
    (Development|PrintString "Switched To gatling guns" true true "(R=0.147565,G=1.000000,B=0.000000,A=1.000000)")))

(event Input|ActionEvents|InputActionFireMainWeapon
  ;[1 1 1] Client Inputs Values
  (:Pressed
    (CallFunction|PlayerMouseDownEvent))
  (:Released
    (CallFunction|PlayerMouseUpEvent)))

(event Input|AxisEvents|InputAxisFire
  (params (AxisValue :type Float%20%28single-precision%29))
  ;[1 1 1] Client Inputs Values
  (if (!= AxisValue 0.0)
    (CallFunction|ShootMainWeapon)))

(event Input|AxisEvents|InputAxisRightThrust
  (params (AxisValue :type Float%20%28single-precision%29))
  ;[1 1 1] Client Inputs Values
  (if (!= AxisValue 0.0)
    (CallFunction|InputLateral AxisValue)))

(event Input|AxisEvents|InputAxisUpThrust
  (params (AxisValue :type Float%20%28single-precision%29))
  ;[1 1 1] Client Inputs Values
  (if (!= AxisValue 0.0)
    (CallFunction|InputVertical AxisValue)))

(event Input|AxisEvents|InputAxisYaw
  (params (AxisValue :type Float%20%28single-precision%29))
  ;[1 1 1] Client Inputs Values
  (if (!= AxisValue 0.0)
    (CallFunction|Yaw AxisValue)))

(event Input|AxisEvents|InputAxisPitch
  (params (AxisValue :type Float%20%28single-precision%29))
  ;[1 1 1] Client Inputs Values
  (if (!= AxisValue 0.0)
    (CallFunction|Pitch AxisValue)))

(event Input|AxisEvents|InputAxisRoll
  (params (AxisValue :type Float%20%28single-precision%29))
  ;[1 1 1] Client Inputs Values
  (if (!= AxisValue 0.0)
    (CallFunction|Roll AxisValue)))

(event Input|AxisEvents|InputAxisForwardThrust
  (params (AxisValue :type Float%20%28single-precision%29))
  ;[1 1 1] Client Inputs Values
  (if true
    (CallFunction|InputForward AxisValue)))

(event Input|KeyboardEvents|Escape
  ;[1 1 1] Client Inputs Values
  (:Pressed
    (bind _returnvalue (UserInterface|CreateWidget "/Game/Widgets/Menu_Escape.Menu_Escape_C"))
    (UserInterface|Viewport|AddtoViewport _returnvalue)
    (Variables|/Script/Engine.PlayerController|SetbShowMouseCursor (Game|GetPlayerController 0) true)))

(event Input|KeyboardEvents|Tab
  ;[1 1 1] Client Inputs Values
  (:Pressed
    (Development|PrintString (Utilities|String|ToString(Integer) (Utilities|Array|Length (Variables|/Game/Blueprints/LevelBlueprints/MyGameInstance.MyGameInstance_C|GetPlayers (Variables|Default|GetGameInstance)))))))

(event Input|KeyboardEvents|SpaceBar
  ;[1 1 1] Client Inputs Values
  (:Pressed
    (CallFunction|StopPlayer)))

(fn ConstructionScript)