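; HUD Blueprint that draws a crosshair showing where the player character is facing.
; Each DrawHUD projects a point far along the character's forward vector to screen space and centers the tinted texture there, so it follows the actor's facing, not the screen center.
; Crosshair size scales with viewport width, and the construction script assigns the texture.
; NewFunction0 is an empty selection switch stub.
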(event EventDrawHUD
  (params (SizeX :type Integer) (SizeY :type Integer))
  (bind _returnvalue (Game|GetPlayerCharacter 0))
  (bind _returnvalue_2 (Transformation|GetWorldLocation _returnvalue))
  (bind _returnvalue_3 (Math|Vector|GetForwardVector _returnvalue))
  (bind _returnvalue_4 (* _returnvalue_3 5e+03))
  (bind _returnvalue_5 (+ _returnvalue_4 _returnvalue_2))
  (bind _returnvalue_6 (Class|HUD|Project _returnvalue_5))
  (bind (_x _y) (Math|Vector|BreakVector _returnvalue_6))
  ;[0 1 0.03408] Start Drawing
  (Utilities|IsValid _returnvalue
    (:Is%20Valid
      ;[1 1 1] Get CrossHair Size
      (Variables|Default|SetCrossHairSize (/ (.x (Viewport|GetViewportSize)) 32.0))
      ;[1 1 1] Draw Crosshair
      (Canvas|DrawTexture (Variables|Default|GetCrossHair) (- _x (/ (Variables|Default|GetCrossHairSize) 2.0)) (- _y (/ (Variables|Default|GetCrossHairSize) 2.0)) (Variables|Default|GetCrossHairSize) (Variables|Default|GetCrossHairSize) 0.0 0.0 1.0 1.0 (Utilities|Struct|MakeLinearColor 1.0 1.0 255.0 1.0) "BLEND_Translucent" 1.0 true))))

(fn ConstructionScript
  (Variables|Default|SetCrossHair "/Game/Textures/CrossHair-Human-001.CrossHair-Human-001"))

(fn NewFunction0
  (params (Selection :type String))
  (switch string Selection
    (:Default
      _)
    (:Case_0
      _)
    (:Case_1
      _))
  (return))