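; Destructible asteroid scene object that floats with gravity disabled and takes damage from hits and damage events.
; MulticastDamage applies the given damage with a fixed impulse along the supplied direction.
; Hits from anything except Player1 apply fixed, impulse-free damage after a short retriggerable delay, so repeated hits restart the timer.
; Each Tick passes the actor's transform to SmoothClientTransform, which sets it directly without interpolation or sweep.
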(event Custom|Smooth%20Client%20Transform
  (params (PlayerTransform :type Transform))
  (Transformation|SetActorTransform PlayerTransform))

(event Custom|Multicast%20Damage
  (params (Damage :type Float%20%28single-precision%29) (Hit%20Position :type Vector) (Impulse%20Dir :type Vector))
  (Game|Damage|ApplyDamage Damage Hit%20Position Impulse%20Dir 5e+02))

(event EventTick
  (params (DeltaSeconds :type Float%20%28single-precision%29))
  (CallFunction|SmoothClientTransform (Transformation|GetActorTransform)))

(event EventHit
  (params (MyComp :type Primitive%20Component%20Object%20Reference) (Other :type Actor%20Object%20Reference) (OtherComp :type Primitive%20Component%20Object%20Reference) (bSelfMoved :type Boolean) (HitLocation :type Vector :default "0, 0, 0") (HitNormal :type Vector :default "0, 0, 0") (NormalImpulse :type Vector :default "0, 0, 0") (Hit :type Hit%20Result%20Structure%20%28by%20ref%29))
  (if (!= Other "/Game/Blueprints/PlayerBlueprints/Player1.Player1")
    (Utilities|FlowControl|RetriggerableDelay 0.2)
    (Game|Damage|ApplyDamage 1e+01 HitLocation HitNormal 0.0)))

(fn ConstructionScript
  (Physics|SetEnableGravity false))